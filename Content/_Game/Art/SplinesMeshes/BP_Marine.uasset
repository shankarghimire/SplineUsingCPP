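; BP_Marine is an actor that travels along the UsefulSpline of a referenced track actor.
; MoveMarine plays the MarineMover timeline, with rate set by Duration and start time by MarineStartOffset.
; Each update maps the timeline alpha to spline distance and sets world location and rotation, with fixed height and yaw offsets.
; BeginPlay is empty and the internal MoveMarine call is unconnected, so nothing here starts the movement.
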(event `self.ReceiveBeginPlay`)

(event `Move Marine`
  (bind _returnvalue (`KismetMathLibrary.Lerp` 0.0 (`SplineComponent.GetSplineLength` (`/Game/SplinesMeshes/BP_SplineTrack.UsefulSpline` (`self.TrackRef`))) (`self.Alpha`)))
  (bind (_returnvalue_x _returnvalue_y _returnvalue_z) (`KismetMathLibrary.BreakVector` (`SplineComponent.GetLocationAtDistanceAlongSpline` (`/Game/SplinesMeshes/BP_SplineTrack.UsefulSpline` (`self.TrackRef`)) _returnvalue "World")))
  (bind (_returnvalue_roll _returnvalue_pitch _returnvalue_yaw) (`KismetMathLibrary.BreakRotator` (`SplineComponent.GetRotationAtDistanceAlongSpline` (`/Game/SplinesMeshes/BP_SplineTrack.UsefulSpline` (`self.TrackRef`)) _returnvalue "World")))
  (`TimelineComponent.SetPlayRate` (`self.MarineMover`) (/ 1.0 (`self.Duration`)))
  (`TimelineComponent.SetNewTime` (`self.MarineMover`) (`self.Marine Start Offset`))
  (bind (_direction _alpha) (`Timeline|MarineMover`)
    (:`Update`
      (set `self.Alpha` _alpha)
      (bind _output_get (set `self.NewActorLocation` (`KismetMathLibrary.MakeVector` _returnvalue_x _returnvalue_y (+ _returnvalue_z 60.0))))
      (bind _output_get_2 (set `self.NewActorRotation` (`KismetMathLibrary.MakeRotator` _returnvalue_roll _returnvalue_pitch (+ _returnvalue_yaw 60.0))))
      (`self.K2_SetActorLocationAndRotation` _output_get _output_get_2))))

(fn `UserConstructionScript`)