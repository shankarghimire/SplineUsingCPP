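; BP_SplineTrack is a spline-driven actor that builds a track from a repeated static mesh at construction time.
; The construction script adds a spline mesh component for each segment between neighboring UsefulSpline points, deforming StaticMesh along ForwardAxis using local start and end positions and tangents.
; Each segment attaches to the spline with query-only collision, and the event graph holds no active logic.
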(fn `UserConstructionScript`
  (for _index (range (+ (- (`SplineComponent.GetNumberOfSplinePoints` (`self.UsefulSpline`)) 2) 1))
    (bind _returnvalue (`AddComponent|NODE_AddSplineMeshComponent-0`))
    (`StaticMeshComponent.SetStaticMesh` _returnvalue (`self.StaticMesh`))
    (`SplineMeshComponent.SetForwardAxis` _returnvalue (`self.Forward Axis`) true)
    (`SceneComponent.K2_AttachToComponent` _returnvalue (`self.UsefulSpline`) "None" "KeepRelative" "KeepRelative" "KeepRelative" true)
    (bind (_location _tangent) (`SplineComponent.GetLocationAndTangentAtSplinePoint` (`self.UsefulSpline`) _index "Local"))
    (bind (_location_2 _tangent_2) (`SplineComponent.GetLocationAndTangentAtSplinePoint` (`self.UsefulSpline`) (+ _index 1) "Local"))
    (`SplineMeshComponent.SetStartAndEnd` _returnvalue _location _tangent _location_2 _tangent_2 true)
    (`PrimitiveComponent.SetCollisionEnabled` _returnvalue "QueryOnly")))