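; BP_Track is a spline-based track actor that places static mesh components at the points of its spline.
; The construction script adds one mesh at the spline point indexed by PointControl.
; At runtime, Tick runs through a one-second Delay, then increments PointControl and adds a mesh at that point, extending the track point by point with no bounds check.
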(event `self.ReceiveTick`
  (params (DeltaSeconds :type "Float (single-precision)"))
  (`KismetSystemLibrary.Delay` 1.0)
  (bind _output_get (set `self.PointControl` (+ (`self.PointControl`) 1)))
  (`AddComponent|NODE_AddStaticMeshComponent-1` :`RelativeTransform` (`KismetMathLibrary.MakeTransform` (`SplineComponent.GetLocationAtSplinePoint` (`self.Spline`) _output_get "Local"))))

(fn `UserConstructionScript`
  (`AddComponent|NODE_AddStaticMeshComponent-0` :`RelativeTransform` (`KismetMathLibrary.MakeTransform` (`SplineComponent.GetLocationAtSplinePoint` (`self.Spline`) (`self.PointControl`) "Local"))))