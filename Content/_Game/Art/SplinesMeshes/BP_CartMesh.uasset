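; BP_CartMesh is an actor built to ride along the spline of a referenced track actor (TrackRef).
; Its MoveBall event plays the BallMover timeline from a start offset, with play rate set by Duration.
; Each update maps the timeline alpha to a distance along the spline and applies that point's world location and rotation to the actor.
; BeginPlay is empty, and the only MoveBall call in the graph is disconnected.
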(event `self.ReceiveBeginPlay`)

(event `Move Ball`
  (bind _returnvalue (`KismetMathLibrary.Lerp` 0.0 (`SplineComponent.GetSplineLength` (`/Game/SplinesMeshes/BP_SplineTrack.UsefulSpline` (`self.TrackRef`))) (`self.Alpha`)))
  (`TimelineComponent.SetPlayRate` (`self.Ball Mover`) (/ 1.0 (`self.Duration`)))
  (`TimelineComponent.SetNewTime` (`self.Ball Mover`) (`self.BallStartOffSet`))
  (bind (_direction _alpha) (`Timeline|Ball Mover`)
    (:`Update`
      (set `self.Alpha` _alpha)
      (`self.K2_SetActorLocationAndRotation` (`SplineComponent.GetLocationAtDistanceAlongSpline` (`/Game/SplinesMeshes/BP_SplineTrack.UsefulSpline` (`self.TrackRef`)) _returnvalue "World") (`SplineComponent.GetRotationAtDistanceAlongSpline` (`/Game/SplinesMeshes/BP_SplineTrack.UsefulSpline` (`self.TrackRef`)) _returnvalue "World")))))

(fn `UserConstructionScript`)